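; BP_Player is the player Blueprint for a voice-driven AI conversation, controlling speech capture through interface events.
; The speak and stop events start and stop capture on its audio component, with a one-second delay after stopping.
; When the player will speak, it asks the HUD to add the view message.
; An unconnected HTTP request to the AI URL would tell the player controller to process the next message.
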(event EventBPIPlayerWillSpeak
  (Class|BPIHud|BPISpeakAllAddtoView(Message) (HUD|GetHUD (Game|GetPlayerController 0)) true))

(event EventBPItoSpeak
  ;[1 1 1] speak and stop
  (Class|AudioGetComp|StartCapture (Variables|Default|GetAudioGetComp)))

(event EventBPIStopSpeak
  ;[1 1 1] speak and stop
  (Class|AudioGetComp|StopCapture (Variables|Default|GetAudioGetComp))
  (Utilities|FlowControl|Delay 1.0))

(fn ConstructionScript)