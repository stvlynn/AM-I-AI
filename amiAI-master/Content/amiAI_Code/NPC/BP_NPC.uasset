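; BP_NPC is a talking historical-figure NPC, with Index selecting Lincoln, Confucius or Einstein.
; The construction script sets mesh and AnimBP, plus separate static heads for Lincoln and Einstein.
; Tick snaps those heads to the head socket and rebuilds answer and vote file paths.
; NPC_Speak imports the chosen local MP3 at runtime, then sends text and duration to the HUD and plays the sound in 2D.
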(event Custom|PlayAudio
  (params (Importer :type Runtime%20Audio%20Importer%20Library%20Object%20Reference) (ImportedSoundWave :type Imported%20Sound%20Wave%20Object%20Reference) (Status :type ERuntimeImportStatus%20Enum :default "SuccessfulImport"))
  ;[1 1 1] find local wav and txt
  (switch Utilities|FlowControl|Switch|SwitchonERuntimeImportStatus Status
    (:SuccessfulImport
      (bind (_content _returnvalue) (Class|WriteLibrary|GetStringinFile (Utilities|Array|Get(acopy) (Variables|Default|GetGetText_Path) (Variables|Default|GetNum))))
      (if _returnvalue
        (Class|BPIHud|BPItoSpeakText(Message) (HUD|GetHUD (Game|GetPlayerController 0)) _content (Class|ImportedSoundWave|GetDurationConst ImportedSoundWave))
        (Audio|PlaySound2D ImportedSoundWave 1.0 1.0 0.0 0 0)))))

(event Custom|SpeakToWidget
  (params (num :type Integer))
  ;[1 1 1] find local wav and txt
  (Variables|Default|SetNum num)
  (bind _returnvalue (Class|RuntimeAudioImporterLibrary|CreateRuntimeAudioImporter))
  (EventDispatchers|BindEventtoOnResult _returnvalue (delegate Custom|PlayAudio))
  (Class|RuntimeAudioImporterLibrary|ImportAudiofromFile _returnvalue (Utilities|Array|Get(acopy) (Variables|Default|GetGetAudio_Path) (Variables|Default|GetNum)) "Mp3"))

(event Custom|NPC_Speak
  (params (num :type Integer))
  (Class|BPIHud|BPISpeakAllAddtoView(Message) (HUD|GetHUD (Game|GetPlayerController 0)) false)
  (CallFunction|SpeaktoWidget num))

(event EventBeginPlay)

(event EventTick
  (params (DeltaSeconds :type Float%20%28single-precision%29))
  (Utilities|FlowControl|Sequence
    (:then_0
      (if (Variables|Default|GetheadisOn_lk)
        (Transformation|SetWorldTransform (Variables|Default|Gethead_lk) (Transformation|GetSocketTransform (Variables|Default|GetSkeletalMesh) "head" "RTS_World") false false)))
    (:then_1
      (if (Variables|Default|GetheadisOn_ayst)
        (Transformation|SetWorldTransform (Variables|Default|Gethead_AYST) (Transformation|GetSocketTransform (Variables|Default|GetSkeletalMesh) "head" "RTS_World") false false)))
    (:then_2
      (switch int (Variables|Default|GetIndex)
        (:1
          (CallFunction|SetArrayGet "lk" "_return.txt" "_to.txt" "林肯-" "回答.mp3" "投票.mp3"))
        (:2
          (CallFunction|SetArrayGet "kz" "_return.txt" "_to.txt" "孔子-" "回答.mp3" "投票.mp3"))
        (:3
          (CallFunction|SetArrayGet "ayst" "_return.txt" "_to.txt" "爱因斯坦-" "回答.mp3" "投票.mp3"))))))

(fn ConstructionScript
  (bind _skeletalmesh (Variables|Default|GetSkeletalMesh))
  (Utilities|FlowControl|Sequence
    (:then_0
      (switch int (Variables|Default|GetIndex)
        (:1
          (Variables|Default|SetInSkeleton "/Game/people/LK/LK2.LK2")
          (Variables|Default|SetABP_Class "/Game/people/LK/ABP_LK2.ABP_LK2_C")
          (Components|StaticMesh|SetStaticMesh (Variables|Default|Gethead_lk) "/Game/people/LK/LKhead3.LKhead3")
          (Variables|Default|SetheadisOn_lk true))
        (:2
          (Variables|Default|SetInSkeleton "/Game/people/KZ/孔子A1.孔子A1")
          (Variables|Default|SetABP_Class "/Game/people/KZ/ABP_KONGZI.ABP_KONGZI_C"))
        (:3
          (Variables|Default|SetInSkeleton "/Game/people/Einstein/IENSTEN.IENSTEN")
          (Variables|Default|SetABP_Class "/Game/people/Einstein/ABP_AYST.ABP_AYST_C")
          (Components|StaticMesh|SetStaticMesh (Variables|Default|Gethead_AYST) "/Game/people/Einstein/IENSTNHead.IENSTNHead")
          (Variables|Default|SetheadisOn_ayst true))))
    (:then_1
      (Variables|/Script/Engine.SkeletalMeshComponent|SetSkeletalMeshAsset _skeletalmesh (Variables|Default|GetInSkeleton))
      (Class|SkeletalMeshComponent|SetAnimClass _skeletalmesh (Variables|Default|GetABP_Class)))))

(fn SetArrayGet
  (params (txt_forward :type String) (txt_return_end :type String) (txt_to_end :type String) (mp3_forward :type String) (mp3_return_end :type String) (mp3_to_end :type String))
  (bind _file (Variables|Default|Getfile))
  (bind _returnvalue (Utilities|String|Append _file mp3_forward))
  (bind _returnvalue_2 (Utilities|String|Append _file txt_forward))
  (Variables|Default|SetGetAudio_Path (Utilities|Array|MakeArray (Utilities|String|Append _returnvalue mp3_return_end) (Utilities|String|Append _returnvalue mp3_to_end)))
  (Variables|Default|SetGetText_Path (Utilities|Array|MakeArray (Utilities|String|Append _returnvalue_2 txt_return_end) (Utilities|String|Append _returnvalue_2 txt_to_end))))