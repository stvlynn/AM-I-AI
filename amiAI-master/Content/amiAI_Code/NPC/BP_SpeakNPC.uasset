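; BP_SpeakNPC plays an NPC's opening and ending lines from local audio and text files, with on-screen text.
; BeginSpeak and EndSpeak briefly delay, message the HUD to show the speech widget, then pick a line by index.
; Runtime Audio Importer loads the MP3 asynchronously.
; On success, the matching text file and audio duration go to the HUD, and the sound plays in 2D.
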(event Custom|PlayAudio
  (params (Importer :type Runtime%20Audio%20Importer%20Library%20Object%20Reference) (ImportedSoundWave :type Imported%20Sound%20Wave%20Object%20Reference) (Status :type ERuntimeImportStatus%20Enum :default "SuccessfulImport"))
  ;[1 1 1] find local wav and txt
  (switch Utilities|FlowControl|Switch|SwitchonERuntimeImportStatus Status
    (:SuccessfulImport
      (bind (_content _returnvalue) (Class|WriteLibrary|GetStringinFile (Utilities|Array|Get(acopy) (Variables|Default|GetGetText_Path) (Variables|Default|GetSpeak%20Num))))
      (if _returnvalue
        (Class|BPIHud|BPItoSpeakText(Message) (HUD|GetHUD (Game|GetPlayerController 0)) _content (Class|ImportedSoundWave|GetDurationConst ImportedSoundWave))
        (Audio|PlaySound2D ImportedSoundWave 1.0 1.0 0.0 0 0)))))

(event Custom|NPC_Speak
  (params (SpeakNum :type Integer))
  ;[1 1 1] find local wav and txt
  (Variables|Default|SetSpeak%20Num SpeakNum)
  (bind _returnvalue (Class|RuntimeAudioImporterLibrary|CreateRuntimeAudioImporter))
  (EventDispatchers|BindEventtoOnResult _returnvalue (delegate Custom|PlayAudio))
  (Class|RuntimeAudioImporterLibrary|ImportAudiofromFile _returnvalue (Utilities|Array|Get(acopy) (Variables|Default|GetGetAudio_Path) (Variables|Default|GetSpeak%20Num)) "Mp3"))

(event Custom|BeginSpeak
  ;[1 1 1] 开场白
  (Utilities|FlowControl|Delay 0.2)
  ;[1 1 1] widget to windows
  (Class|BPIHud|BPISpeakAllAddtoView(Message) (HUD|GetHUD (Game|GetPlayerController 0)) false)
  ;[1 1 1] 音频和文本位置
  (CallFunction|NPCSpeak))

(event Custom|EndSpeak
  (Utilities|FlowControl|Delay 0.2)
  ;[1 1 1] widget to windows
  (Class|BPIHud|BPISpeakAllAddtoView(Message) (HUD|GetHUD (Game|GetPlayerController 0)) false)
  ;[1 1 1] 音频和文本位置
  (CallFunction|NPCSpeak 1))

(fn ConstructionScript)